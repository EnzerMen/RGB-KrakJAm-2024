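; BP_ToyPartRandomizer picks a random toy part by weight from the ToySetWeight map.
; BeginPlay totals the map's values into WeightSum.
; GetRandomToyPart rolls an integer up to that sum, walks the cumulative weights until one reaches the roll, then returns the key at that index.
; The roll includes both zero and the sum, so the first entry gets one extra chance.
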(event EventBeginPlay
  (bind _values (Utilities|Map|Values (Variables|Default|GetToySetWeight)))
  (for _array_element _values
    (Variables|Default|SetWeightSum (+ (Variables|Default|GetWeightSum) _array_element))))

(fn ConstructionScript)

(fn GetRandomToyPart
  (LocalVariables|SetRandomizedWeight (Math|Random|RandomIntegerinRange 0 (Variables|Default|GetWeightSum)))
  (LocalVariables|SetLoopWeight 0)
  (bind _values (Utilities|Map|Values (Variables|Default|GetToySetWeight)))
  (bind (_array_element _array_index) (Utilities|Array|ForEachLoopwithBreak _values :!label _label)
    (:LoopBody
      (bind _output_get (LocalVariables|SetLoopWeight (+ _array_element (LocalVariables|GetLoopWeight))))
      (if (<= (LocalVariables|GetRandomizedWeight) _output_get)
        (bind _output_get_2 (LocalVariables|SetIndexNumber _array_index))
        (goto _label Break)))
    (:Completed
      (bind _keys (Utilities|Map|Keys (Variables|Default|GetToySetWeight)))
      (return (Utilities|Array|Get(acopy) _keys (LocalVariables|GetIndexNumber))))))