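; End-game spawner that presents the player's completed toys, then closes out the game.
; When StartSpawning is called, a delayed loop walks the CompleteToys array on MainGameMode, teleporting each existing toy to the spawner's transform and unhiding it.
; After the last toy, it shows the WBP_Thanks widget and, following a short delay, opens the MainMenu level.
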(event Custom|StartSpawning
  (Development|PrintString "Start Spawning")
  (bind _index (Utilities|ForLoopwithDelay 0 (- (Utilities|Array|Length (Variables|/Game/Blueprints/MainGameMode.MainGameMode_C|GetCompleteToys (Variables|Default|GetAs%20Main%20Game%20Mode))) 1) 5.0)
    (:LoopBody
      (Transformation|SetWorldTransform (Variables|/Script/Engine.Actor|GetRootComponent (Utilities|Array|Get(acopy) (Variables|/Game/Blueprints/MainGameMode.MainGameMode_C|GetCompleteToys (Variables|Default|GetAs%20Main%20Game%20Mode)) _index)) (Transformation|GetActorTransform) false true)
      (Rendering|SetActorHiddenInGame (Utilities|Array|Get(acopy) (Variables|/Game/Blueprints/MainGameMode.MainGameMode_C|GetCompleteToys (Variables|Default|GetAs%20Main%20Game%20Mode)) _index) false))
    (:Completed
      (Utilities|FlowControl|Delay 5.0)
      (bind _returnvalue (UserInterface|CreateWidget "/Game/Blueprints/Widgets/WBP_Thanks.WBP_Thanks_C"))
      (UserInterface|Viewport|AddtoViewport _returnvalue 0)
      (Utilities|FlowControl|Delay 5.0)
      (Game|OpenLevel(byName) "MainMenu"))))

(event EventBeginPlay
  (bind _asmain_game_mode (Utilities|Casting|CastToMainGameMode (Game|GetGameMode)))
  (Variables|Default|SetAs%20Main%20Game%20Mode _asmain_game_mode))

(fn ConstructionScript)