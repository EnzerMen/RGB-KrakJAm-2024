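; Conveyor belt actor, apparently for the credits, that carries BP_Toy actors along and displays their names.
; Each tick it offsets every toy overlapping Box along the Arrow's forward vector, scaled by Speed and delta time, without sweeping.
; When a toy enters ShowNameBox, its ToyData name is passed to the WBP_BaseText in the Widget component to show.
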(event OnComponentBeginOverlap(ShowNameBox)
  (params (OverlappedComponent :type Primitive%20Component%20Object%20Reference) (OtherActor :type Actor%20Object%20Reference) (OtherComp :type Primitive%20Component%20Object%20Reference) (OtherBodyIndex :type Integer) (bFromSweep :type Boolean) (SweepResult :type Hit%20Result%20Structure%20%28by%20ref%29))
  (bind _asbp_toy (Utilities|Casting|CastToBP_Toy OtherActor))
  (Default|ShowMe (.AsWBP%20Base%20Text (Utilities|Casting|CastToWBP_BaseText (UserInterface|GetWidget (Variables|Default|GetWidget)))) (Utilities|Text|ToText(String) (.toyname (Variables|/Game/Blueprints/MapObjects/BP_Toy.BP_Toy_C|GetToyData _asbp_toy)))))

(event EventTick
  (params (DeltaSeconds :type Float%20%28single-precision%29))
  (for _array_element (Collision|GetOverlappingActors (Variables|Default|GetBox) "/Game/Blueprints/MapObjects/BP_Toy.BP_Toy_C" :!class /Script/Engine.PrimitiveComponent)
    (Transformation|AddActorWorldOffset _array_element (* (* DeltaSeconds (Variables|Default|GetSpeed)) (Math|Vector|GetForwardVector (Variables|Default|GetArrow))))))

(fn ConstructionScript)