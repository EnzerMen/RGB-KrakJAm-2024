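; End-game map actor that reveals the completed toys stored in the main game mode at its own position.
; BeginPlay caches the game mode and sets a one-shot timer, with no bound event shown.
; StartSpawning loops over the toys, teleporting each to the spawner's transform and unhiding it.
; A Delay sits inside the plain for loop, so it does not stagger the iterations.
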(event Custom|StartSpawning
  (Development|PrintString "Start Spawning")
  (for _index (range 0 (- (Utilities|Array|Length (Variables|/Game/Blueprints/MainGameMode.MainGameMode_C|GetCompleteToys (Variables|Default|GetAs%20Main%20Game%20Mode))) 1))
    (Transformation|SetWorldTransform (Variables|/Script/Engine.Actor|GetRootComponent (Utilities|Array|Get(acopy) (Variables|/Game/Blueprints/MainGameMode.MainGameMode_C|GetCompleteToys (Variables|Default|GetAs%20Main%20Game%20Mode)) _index)) (Transformation|GetActorTransform) false true)
    (Rendering|SetActorHiddenInGame (Utilities|Array|Get(acopy) (Variables|/Game/Blueprints/MainGameMode.MainGameMode_C|GetCompleteToys (Variables|Default|GetAs%20Main%20Game%20Mode)) _index) false)
    (Utilities|FlowControl|Delay 2.0)))

(event EventBeginPlay
  (bind _asmain_game_mode (Utilities|Casting|CastToMainGameMode (Game|GetGameMode)))
  (Variables|Default|SetAs%20Main%20Game%20Mode _asmain_game_mode)
  (Utilities|Time|SetTimerbyEvent 0 1e+01))

(fn ConstructionScript)