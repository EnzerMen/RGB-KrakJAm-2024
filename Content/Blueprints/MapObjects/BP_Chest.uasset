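; BP_Chest is an interactable chest that holds a growing inventory of random toy parts.
; It fills up at BeginPlay, then a self-restarting random-delay timer adds another part and refreshes the inventory widget.
; GetRandomPart asks BP_ToyPartRandomizer for a toy set and takes the first matching DataTable row.
; Interacting empty-handed puts the character in UI mode and opens WBP_Inventory, created on first use in the Widget component.
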(event Custom|AddNewItem
  (bind _foundtoypart (CallFunction|GetRandomPart))
  (Utilities|Array|Add (Variables|Private|GetToyParts) _foundtoypart)
  (Utilities|FlowControl|Sequence
    (:then_0
      (Utilities|Time|SetTimerbyEvent (delegate Custom|AddNewItem) (Math|Random|RandomFloatinRange (Variables|ChestSettings|GetMinTimeDelay) (Variables|ChestSettings|GetMaxTimeDelay))))
    (:then_1
      (CallFunction|UpdateInventory))))

(event EventBeginPlay
  (Utilities|FlowControl|Sequence
    (:then_0
      (bind _returnvalue (Actor|GetActorOfClass "/Game/Blueprints/MapObjects/BP_ToyPartRandomizer.BP_ToyPartRandomizer_C"))
      (Variables|Private|SetToyPartRandomizer _returnvalue)
      (for _index (range 0 10)
        (bind _foundtoypart (CallFunction|GetRandomPart))
        (Utilities|Array|Add (Variables|Private|GetToyParts) _foundtoypart)))
    (:then_1
      (Utilities|Time|SetTimerbyEvent (delegate Custom|AddNewItem) (Math|Random|RandomFloatinRange (Variables|ChestSettings|GetMinTimeDelay) (Variables|ChestSettings|GetMaxTimeDelay))))))

(fn ConstructionScript)

(fn OpenInventoryWidget
  (params (Character :type Character%20Object%20Reference))
  (bind _widget (Variables|Default|GetWidget))
  (bind _returnvalue (UserInterface|GetWidget _widget))
  ;[1 1 1] IfValid-Return
  (Utilities|IsValid _returnvalue
    (:Is%20Valid
      (return (.AsWBP%20Inventory (Utilities|Casting|CastToWBP_Inventory _returnvalue))))
    (:Is%20Not%20Valid
      ;[1 1 1] IfNotValid-Create
      (bind _asplayer_controller (Utilities|Casting|CastToPlayerController (Pawn|GetController Character)))
      (bind _returnvalue_2 (UserInterface|CreateWidget "/Game/Blueprints/Widgets/WBP_Inventory.WBP_Inventory_C" _asplayer_controller))
      (UserInterface|SetWidget (Variables|Default|GetWidget) _returnvalue_2)
      (return _returnvalue_2))))

(fn GetRandomPart
  (bind _datatable (Variables|ChestSettings|GetDataTable))
  (bind _randomtoyset (Default|GetRandomToySet (Variables|Private|GetToyPartRandomizer)))
  (LocalVariables|SetRandomizedSet _randomtoyset)
  (bind _outrownames (DataTable|GetDataTableRowNames _datatable))
  (bind _array_element (Utilities|Array|ForEachLoopwithBreak _outrownames :!label _label)
    (:LoopBody
      (bind _returnvalue (Utilities|GetDataTableRow _datatable _array_element)
        (:then
          (if (Utilities|Enum|Equal(Enum) (.ToySet (Utilities|Struct|BreakS_ToyPartData _returnvalue)) (LocalVariables|GetRandomizedSet))
            (LocalVariables|SetFoundPart _returnvalue)
            (goto _label Break)))))
    (:Completed
      (Utilities|IsValid (.staticmesh (LocalVariables|GetFoundPart))
        (:Is%20Valid
          (return (LocalVariables|GetFoundPart)))
        (:Is%20Not%20Valid
          (CallFunction|GetRandomPart))))))

(fn UpdateInventory
  (bind _widget (Variables|Default|GetWidget))
  (bind _returnvalue (UserInterface|GetWidget _widget))
  (bind _aswbp_inventory (Utilities|Casting|CastToWBP_Inventory _returnvalue))
  (Utilities|IsValid _returnvalue
    (:Is%20Valid
      (Default|UpdateInventory _aswbp_inventory (Variables|Private|GetToyParts) false)
      (Default|ActivateCurrentSlot _aswbp_inventory))))

(fn Interact
  (params (Character :type BP%20Player%20Character%20Object%20Reference) (IsHoldingItem :type Boolean))
  (if (not IsHoldingItem)
    (Variables|/Game/Blueprints/Player/BP_PlayerCharacter.BP_PlayerCharacter_C|SetUI_Mode Character true)
    (bind _inventorywidget (CallFunction|OpenInventoryWidget Character))
    (Default|OpenInventory _inventorywidget self)
    (return)))