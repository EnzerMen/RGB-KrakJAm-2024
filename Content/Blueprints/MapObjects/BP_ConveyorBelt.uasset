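; BP_ConveyorBelt is a map object that turns a player's held item into a toy and carries it along the belt.
; Interact, if the belt is not occupied, spawns a BP_Toy facing the arrow at the player's X, initializes it with the held part, then destroys that item.
; Tick moves every overlapping toy along the arrow's forward vector at Speed, without sweeping.
; Nothing here clears Occupied once set.
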(event EventTick
  (params (DeltaSeconds :type Float%20%28single-precision%29))
  (for _array_element (Collision|GetOverlappingActors (Variables|Default|GetBox) "/Game/Blueprints/MapObjects/BP_Toy.BP_Toy_C" :!class /Script/Engine.PrimitiveComponent)
    (Transformation|AddActorWorldOffset _array_element (* (* DeltaSeconds (Variables|Default|GetSpeed)) (Math|Vector|GetForwardVector (Variables|Default|GetArrow))))))

(fn ConstructionScript)

(fn RemoveHoldItem
  (params (Player :type BP%20Player%20Character%20Object%20Reference))
  (Variables|/Game/Blueprints/Player/BP_PlayerCharacter.BP_PlayerCharacter_C|SetIsHoldingItem Player false)
  (Actor|DestroyActor (Variables|/Game/Blueprints/Player/BP_PlayerCharacter.BP_PlayerCharacter_C|GetHoldItem Player)))

(fn Interact
  (params (Character :type BP%20Player%20Character%20Object%20Reference) (IsHoldingItem :type Boolean))
  (bind _self self)
  (bind _returnvalue (Transformation|GetActorLocation _self))
  (if (and IsHoldingItem (not (Variables|Default|GetOccupied)))
    (Utilities|FlowControl|Sequence
      (:then_0
        (bind _returnvalue_2 (Game|SpawnActorfromClass "/Game/Blueprints/MapObjects/BP_Toy.BP_Toy_C" (Math|Transform|MakeTransform (Math|Vector|MakeVector (.x (Transformation|GetWorldLocation (Variables|/Script/Engine.Character|GetCapsuleComponent Character))) (.y _returnvalue) (+ (.z _returnvalue) 5.0)) (Math|Conversions|RotationFromXVector (Math|Vector|GetForwardVector (Variables|Default|GetArrow))) "1.000000,1.000000,1.000000") "Undefined" "MultiplyWithRoot" 0 0))
        (Default|AddNewPart _returnvalue_2 (Variables|/Game/Blueprints/MapObjects/BP_ToyPart.BP_ToyPart_C|GetToyPartData (Variables|/Game/Blueprints/Player/BP_PlayerCharacter.BP_PlayerCharacter_C|GetHoldItem Character)))
        (Default|InitializeToy _returnvalue_2)
        (Variables|Default|SetOccupied true))
      (:then_1
        (CallFunction|RemoveHoldItem Character))
      (:then_2
        (return)))))