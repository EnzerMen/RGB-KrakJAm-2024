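; BP_TestRandomName is a test Blueprint that sets up two-player word selection from adjective and noun data tables.
; On BeginPlay it creates P1 and P2 word widgets, both owned by player 0's controller, adds them to the viewport and caches their selection sub-widgets.
; A short one-shot timer then initializes P1 with adjectives and P2 with nouns, each with its own word index.
; ShowWidgets is an empty stub.
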(event Custom|OpenWidgets
  (Default|Initialize (Variables|Default|GetSelectionP1) "/Game/Data/DataBase/DT_Adjective.DT_Adjective")
  (Default|Initialize (Variables|Default|GetSelectionP2) "/Game/Data/DataBase/DT_Noun.DT_Noun" 1))

(event EventBeginPlay
  (Utilities|Time|SetTimerbyEvent (delegate Custom|OpenWidgets) 2.0)
  (bind _returnvalue (UserInterface|CreateWidget "/Game/Blueprints/Widgets/WBP_WordWidget_P1.WBP_WordWidget_P1_C" (.AsBP%20Player%20Controller (Utilities|Casting|CastToBP_PlayerController (Pawn|GetController (Game|Player|GetPlayerPawn 0))))))
  (Variables|Default|SetSelectionP1 (Variables|/Game/Blueprints/Widgets/WBP_WordWidget_P1.WBP_WordWidget_P1_C|GetWBP_Selection _returnvalue))
  (UserInterface|Viewport|AddtoViewport _returnvalue 0)
  (bind _returnvalue_2 (UserInterface|CreateWidget "/Game/Blueprints/Widgets/WBP_WordWidget_P2.WBP_WordWidget_P2_C" (.AsBP%20Player%20Controller (Utilities|Casting|CastToBP_PlayerController (Pawn|GetController (Game|Player|GetPlayerPawn 0))))))
  (Variables|Default|SetSelectionP2 (Variables|/Game/Blueprints/Widgets/WBP_WordWidget_P2.WBP_WordWidget_P2_C|GetWBP_Selection _returnvalue_2))
  (UserInterface|Viewport|AddtoViewport _returnvalue_2 0))

(fn ConstructionScript)

(fn ShowWidgets)