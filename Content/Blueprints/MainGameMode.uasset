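; MainGameMode is the game mode that runs the end-of-game sequence through a BeginEndGame event.
; The event plays the FadeOutFadeIn level sequence, then after a delay switches the first player's view to the actor tagged "cam2".
; After a second delay it starts the BP_EndGameToySpawner spawning and adds the WBP_Ending widget to the viewport.
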(event Custom|BeginEndGame
  (bind _outactor (Sequencer|Player|CreateLevelSequencePlayer "/Game/Sequences/FadeOutFadeIn.FadeOutFadeIn"))
  (Sequencer|Player|Play (Variables|/Script/LevelSequence.LevelSequenceActor|GetSequencePlayer _outactor) :!class /Script/MovieScene.MovieSceneSequencePlayer)
  (Utilities|FlowControl|Delay 2.0)
  (Development|PrintString "Koniec Sie zacyzna")
  (bind _outactors (Actor|GetAllActorswithTag "cam2"))
  (Game|Player|SetViewTargetwithBlend (Game|GetPlayerController 0) (Utilities|Array|Get(acopy) _outactors) 0.0 "VTBlend_Linear" 0.0 false)
  (Utilities|FlowControl|Delay 2.0)
  (bind _returnvalue (Actor|GetActorOfClass "/Game/Blueprints/MapObjects/BP_EndGameToySpawner.BP_EndGameToySpawner_C"))
  (Default|StartSpawning _returnvalue)
  (bind _returnvalue_2 (UserInterface|CreateWidget "/Game/Blueprints/Widgets/WBP_Ending.WBP_Ending_C"))
  (UserInterface|Viewport|AddtoViewport _returnvalue_2 0))

(event EventBeginPlay)

(event EventTick
  (params (DeltaSeconds :type Float%20%28single-precision%29)))

(fn ConstructionScript)