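; BP_GetRandomNames runs a two-player word pick that builds a combined name for BP_Cheesomate.
; On BeginPlay, after a short delay, it creates a word widget for each player.
; OpenWidgets resets readiness, puts both characters in UI mode and feeds adjectives to player one and nouns to player two.
; CheckPlayerReadines waits until both are ready, exits UI mode, collapses the widgets and passes the joined words to BP_Cheesomate's CalculateAndStuff.
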(event Custom|OpenWidgets
  (Variables|Default|SetP1_Ready false)
  (Variables|Default|SetP2_Ready false)
  (bind _asbp_player_character (Utilities|Casting|CastToBP_PlayerCharacter (Game|Player|GetPlayerPawn 0)))
  (Variables|/Game/Blueprints/Player/BP_PlayerCharacter.BP_PlayerCharacter_C|SetUI_Mode _asbp_player_character true)
  (Default|Initialize (Variables|Default|GetSelectionP1) "/Game/Data/DataBase/DT_Adjective.DT_Adjective")
  (bind _asbp_player_character_2 (Utilities|Casting|CastToBP_PlayerCharacter (Game|Player|GetPlayerPawn 1)))
  (Variables|/Game/Blueprints/Player/BP_PlayerCharacter.BP_PlayerCharacter_C|SetUI_Mode _asbp_player_character_2 true)
  (Default|Initialize (Variables|Default|GetSelectionP2) "/Game/Data/DataBase/DT_Noun.DT_Noun" 1 1)
  (Default|Show (Variables|Default|GetMainSelectionP1)))

(event Custom|CheckPlayerReadines
  (if (and (Variables|Default|GetP1_Ready) (Variables|Default|GetP2_Ready))
    (Utilities|FlowControl|Sequence
      (:then_0
        (bind _asbp_player_character (Utilities|Casting|CastToBP_PlayerCharacter (Game|Player|GetPlayerPawn 0)))
        (Variables|/Game/Blueprints/Player/BP_PlayerCharacter.BP_PlayerCharacter_C|SetUI_Mode _asbp_player_character false)
        (bind _asbp_player_character_2 (Utilities|Casting|CastToBP_PlayerCharacter (Game|Player|GetPlayerPawn 1)))
        (Variables|/Game/Blueprints/Player/BP_PlayerCharacter.BP_PlayerCharacter_C|SetUI_Mode _asbp_player_character_2 false)
        (Default|Collapse (Variables|Default|GetSelectionP2))
        (Default|Collapse (Variables|Default|GetSelectionP1))
        (Default|Collapse (Variables|Default|GetMainSelectionP1)))
      (:then_1
        (bind _output_get (Variables|Default|SetFinalName (Utilities|Text|ToText(String) (Utilities|String|Append (Utilities|String|ToString(Text) (Variables|Default|GetWord_1)) " " (Utilities|String|ToString(Text) (Variables|Default|GetWord_2))))))
        (bind _returnvalue (Actor|GetActorOfClass "/Game/Blueprints/MapObjects/BP_Cheesomate.BP_Cheesomate_C"))
        (Default|CalculateandStuff _returnvalue _output_get)))))

(event EventBeginPlay
  (Utilities|FlowControl|Delay 0.2)
  (Utilities|FlowControl|Sequence
    (:then_0
      (bind _asplayer_controller (Utilities|Casting|CastToPlayerController (Pawn|GetController (Game|Player|GetPlayerPawn 0))))
      (bind _returnvalue (UserInterface|CreateWidget "/Game/Blueprints/Widgets/WBP_WordWidget_P1.WBP_WordWidget_P1_C" _asplayer_controller))
      (Variables|Default|SetMainSelectionP1 _returnvalue)
      (Variables|Default|SetSelectionP1 (Variables|/Game/Blueprints/Widgets/WBP_WordWidget_P1.WBP_WordWidget_P1_C|GetWBP_Selection _returnvalue))
      (UserInterface|Viewport|AddtoViewport _returnvalue 0)
      (bind _asplayer_controller_2 (Utilities|Casting|CastToPlayerController (Pawn|GetController (Game|Player|GetPlayerPawn 1))))
      (bind _returnvalue_2 (UserInterface|CreateWidget "/Game/Blueprints/Widgets/WBP_WordWidget_P2.WBP_WordWidget_P2_C" _asplayer_controller_2))
      (Variables|Default|SetSelectionP2 (Variables|/Game/Blueprints/Widgets/WBP_WordWidget_P2.WBP_WordWidget_P2_C|GetWBP_Selection _returnvalue_2))
      (UserInterface|Viewport|AddtoViewport _returnvalue_2 0))))

(fn ConstructionScript)

(fn ShowWidgets)