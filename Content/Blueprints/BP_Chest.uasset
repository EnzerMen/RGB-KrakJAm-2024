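; BP_Chest is an interactable chest that shows a randomly sized item list in an inventory widget.
; On BeginPlay it fills ItemList with stringified loop indices as item entries, with the count randomized.
; Interact passes that list to WBP_Inventory's OpenInventory.
; GetWidget lazily creates the inventory widget for the interacting character's player controller, stores it in the Widget component and reuses it afterwards.
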(event EventBeginPlay
  (for _index (range 0 (Math|Random|RandomIntegerinRange 1 6))
    (Utilities|Array|Add (Variables|Default|GetItemList) (Utilities|String|ToString(Integer) _index))))

(fn ConstructionScript)

(fn GetWidget
  (params (Character :type Character%20Object%20Reference))
  (bind _widget (Variables|Default|GetWidget))
  (bind _returnvalue (UserInterface|GetWidget _widget))
  (Utilities|IsValid _returnvalue
    (:Is%20Valid
      (return (.AsWBP%20Inventory (Utilities|Casting|CastToWBP_Inventory _returnvalue))))
    (:Is%20Not%20Valid
      (bind _asplayer_controller (Utilities|Casting|CastToPlayerController (Pawn|GetController Character)))
      (bind _returnvalue_2 (UserInterface|CreateWidget "/Game/Blueprints/Widgets/WBP_Inventory.WBP_Inventory_C" _asplayer_controller))
      (UserInterface|SetWidget (Variables|Default|GetWidget) _returnvalue_2)
      (return _returnvalue_2))))

(fn Interact
  (params (Character :type BP%20Player%20Character%20Object%20Reference))
  (bind _inventorywidget (CallFunction|GetWidget Character))
  (Default|OpenInventory _inventorywidget (Variables|Default|GetItemList))
  (return true))