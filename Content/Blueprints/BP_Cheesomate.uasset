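; BP_Cheesomate scores a four-part toy with poker-style bonus multipliers.
; CalculateSetMultiplier compares the parts' sets for flush, three of a kind, two pair or pair.
; CalculatePartMultiplier counts torso, legs, arms and head parts in their matching slots, up to a straight ("Strit") bonus.
; BeginPlay computes both and prints them, while OverlapTemp only copies ToyData from Toy without recalculating.
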(event Custom|OverlapTemp
  (Variables|Default|SetToy%20Data (Variables|/Game/Blueprints/BP_Toy.BP_Toy_C|GetToyData (Variables|Default|GetToy))))

(event EventBeginPlay
  (CallFunction|CalculateSetMultiplier)
  (Development|PrintString (Utilities|String|ToString(Float) (Variables|Default|GetSetMultiplier)))
  (CallFunction|CalculatePartMultiplier)
  (Development|PrintString (Utilities|String|ToString(Float) (Variables|Default|GetPartMultiplier))))

(fn ConstructionScript)

(fn CalculateSetMultiplier
  (bind _toy_data (Variables|Default|GetToy%20Data))
  (bind _toypartdata (Utilities|Struct|BreakS_ToyData _toy_data))
  (bind _output (Utilities|Array|Get(acopy) _toypartdata 3))
  (bind _output_2 (Utilities|Array|Get(acopy) _toypartdata))
  (bind _output_3 (Utilities|Array|Get(acopy) _toypartdata 1))
  (bind _output_4 (Utilities|Array|Get(acopy) _toypartdata 2))
  (bind _returnvalue (Utilities|Enum|Equal(Enum) (.toyset _output_3) (.toyset _output_4)))
  (bind _returnvalue_2 (Utilities|Enum|Equal(Enum) (.toyset _output_3) (.toyset _output)))
  (bind _returnvalue_3 (Utilities|Enum|Equal(Enum) (.toyset _output_4) (.toyset _output)))
  (bind _returnvalue_4 (Utilities|Enum|Equal(Enum) (.toyset _output_2) (.toyset _output_3)))
  (bind _returnvalue_5 (Utilities|Enum|Equal(Enum) (.toyset _output_2) (.toyset _output_3)))
  (bind _returnvalue_6 (Utilities|Enum|Equal(Enum) (.toyset _output_2) (.toyset _output_4)))
  (bind _returnvalue_7 (Utilities|Enum|Equal(Enum) (.toyset _output_2) (.toyset _output)))
  ;[1 1 1] Flush
  (if (Math|Boolean|ANDBoolean (Utilities|Enum|Equal(Enum) (.toyset _output_2) (.toyset _output_3)) (Utilities|Enum|Equal(Enum) (.toyset _output_3) (.toyset _output_4)) (Utilities|Enum|Equal(Enum) (.toyset _output_4) (.toyset _output)))
    (Variables|Default|SetSetMultiplier (LocalVariables|GetFlushBonus))
    (else
      ;[1 1 1] Three of a kind
      (if (Math|Boolean|ORBoolean (and _returnvalue_4 (Utilities|Enum|Equal(Enum) (.toyset _output_2) (.toyset _output_4))) (and _returnvalue_4 (Utilities|Enum|Equal(Enum) (.toyset _output_2) (.toyset _output))) (and (Utilities|Enum|Equal(Enum) (.toyset _output_3) (.toyset _output_4)) (Utilities|Enum|Equal(Enum) (.toyset _output_3) (.toyset _output))) (and (Utilities|Enum|Equal(Enum) (.toyset _output) (.toyset _output_2)) (Utilities|Enum|Equal(Enum) (.toyset _output_4) (.toyset _output))))
        (Variables|Default|SetSetMultiplier (LocalVariables|GetToakBonus))
        (else
          ;[1 1 1] Two Pair
          (if (Math|Boolean|ORBoolean (and _returnvalue_5 _returnvalue_3) (and _returnvalue _returnvalue_7) (and _returnvalue_6 _returnvalue_2))
            (Variables|Default|SetSetMultiplier (LocalVariables|GetTwoPairBonus))
            (else
              ;[1 1 1] Pair
              (if (Math|Boolean|ORBoolean _returnvalue_5 _returnvalue_6 _returnvalue_7 _returnvalue _returnvalue_2 _returnvalue_3)
                (Variables|Default|SetSetMultiplier (LocalVariables|GetPairBonus))
                (else
                  (Variables|Default|SetSetMultiplier 1.0))))))))))

(fn CalculatePartMultiplier
  (bind _toy_data (Variables|Default|GetToy%20Data))
  (bind _toypartdata (Utilities|Struct|BreakS_ToyData _toy_data))
  (for _index (range 0 3)
    (switch int _index
      (:0
        (if (Utilities|Enum|Equal(Enum) (.toypart (Utilities|Array|Get(acopy) _toypartdata)) "NewEnumerator1")
          (LocalVariables|SetValidParts (+ 1 (LocalVariables|GetValidParts)) :!label _label)))
      (:1
        (if (Utilities|Enum|Equal(Enum) (.toypart (Utilities|Array|Get(acopy) _toypartdata 1)) "NewEnumerator3")
          (goto _label)))
      (:2
        (if (Utilities|Enum|Equal(Enum) (.toypart (Utilities|Array|Get(acopy) _toypartdata 2)) "NewEnumerator2")
          (goto _label)))
      (:3
        (if (Utilities|Enum|Equal(Enum) (.toypart (Utilities|Array|Get(acopy) _toypartdata 3)) "NewEnumerator0")
          (goto _label)))))
  (switch int (LocalVariables|GetValidParts)
    (:0
      (Variables|Default|SetPartMultiplier 0.8))
    (:1
      (Variables|Default|SetPartMultiplier (LocalVariables|GetOnePartBonus)))
    (:2
      (Variables|Default|SetPartMultiplier (LocalVariables|GetTwoPartBonus)))
    (:3
      (Variables|Default|SetPartMultiplier (LocalVariables|GetThreePartBonus)))
    (:4
      (Variables|Default|SetPartMultiplier (LocalVariables|GetStritBonus)))))